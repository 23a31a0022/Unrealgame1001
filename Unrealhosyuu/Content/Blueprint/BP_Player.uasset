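; Player character with Enhanced Input movement, camera-relative hitscan shooting at BP_Enemy, door interaction and UI.
; Shooting requires HasGun, decrements Ammo without an empty check and broadcasts the change.
; V toggles first- and third-person cameras, changing head opacity through a dynamic material.
; Damage clamps Health and flashes a widget; death disables input, sets a Ragdoll collision profile without physics simulation, and shows game over.
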(event Custom|ShowInteract
  (params (IsDoorLocked :type Boolean))
  (bind _returnvalue (UserInterface|CreateWidget "/Game/UI/WBP_Interact.WBP_Interact_C"))
  (bind _output_get (Variables|Default|SetUI_Interact _returnvalue))
  (UserInterface|Viewport|AddtoViewport _output_get 0)
  (if IsDoorLocked
    (Variables|/Script/UMG.TextBlock|SetText (Variables|/Game/UI/WBP_Interact.WBP_Interact_C|GetTxt_Message (Variables|Default|GetUI_Interact)) "鍵がかかっている")
    (else
      (Variables|/Script/UMG.TextBlock|SetText (Variables|/Game/UI/WBP_Interact.WBP_Interact_C|GetTxt_Message (Variables|Default|GetUI_Interact)) "Ｅキーでインタラクト"))))

(event Custom|HideInteract
  (Widget|RemovefromParent (Variables|Default|GetUI_Interact)))

(event Input|EnhancedActionEvents|EnhancedInputActionIA_MyMove
  (params (ActionValue :type Vector%202D%20Structure) (ElapsedSeconds :type Float%20%28double-precision%29) (TriggeredSeconds :type Float%20%28double-precision%29) (InputAction :type Input%20Action%20Object%20Reference :default "/Game/Input/IA_MyMove.IA_MyMove"))
  (bind _returnvalue (Pawn|GetControlRotation :!class /Script/Engine.Pawn))
  (bind _yaw (Math|Rotator|BreakRotator _returnvalue))
  (bind _returnvalue_2 (Math|Rotator|MakeRotator 0.0 0.0 _yaw))
  (Pawn|Input|AddMovementInput (Math|Vector|GetForwardVector _returnvalue_2) (.y ActionValue) false)
  (Pawn|Input|AddMovementInput (Math|Vector|GetRightVector _returnvalue_2) (.x ActionValue) false))

(event Input|EnhancedActionEvents|EnhancedInputActionIA_MyLook
  (params (ActionValue :type Vector%202D%20Structure) (ElapsedSeconds :type Float%20%28double-precision%29) (TriggeredSeconds :type Float%20%28double-precision%29) (InputAction :type Input%20Action%20Object%20Reference :default "/Game/Input/IA_MyLook.IA_MyLook"))
  (Pawn|Input|AddControllerYawInput (.x ActionValue))
  (Pawn|Input|AddControllerPitchInput (.y ActionValue)))

(event Input|EnhancedActionEvents|EnhancedInputActionIA_MyShoot
  (params (ActionValue :type Boolean) (ElapsedSeconds :type Float%20%28double-precision%29) (TriggeredSeconds :type Float%20%28double-precision%29) (InputAction :type Input%20Action%20Object%20Reference :default "/Game/Input/IA_MyShoot.IA_MyShoot"))
  (bind _returnvalue (Game|GetPlayerCameraManager 0))
  (bind _returnvalue_2 (Camera|GetCameraLocation _returnvalue))
  (:Started
    (if (Variables|Default|GetHasGun)
      (bind _outhit (Collision|LineTraceByChannel _returnvalue_2 (+ _returnvalue_2 (* (Math|Vector|GetForwardVector (Camera|GetCameraRotation _returnvalue)) 1e+04)) "TraceTypeQuery1" false 0 "None"))
      (bind _output_get (Variables|Default|SetAmmo (Variables|Default|GetAmmo)))
      (bind _output_get_2 (Variables|Default|SetAmmo (- _output_get 1)))
      (Default|CallOnAmmoChanged _output_get_2)
      (bind _asbp_enemy (Utilities|Casting|CastToBP_Enemy (.HitActor (Collision|BreakHitResult _outhit))))
      (Default|TakeDamage _asbp_enemy))))

(event Input|EnhancedActionEvents|EnhancedInputActionIA_MyInteract
  (params (ActionValue :type Boolean) (ElapsedSeconds :type Float%20%28double-precision%29) (TriggeredSeconds :type Float%20%28double-precision%29) (InputAction :type Input%20Action%20Object%20Reference :default "/Game/Input/IA_MyInteract.IA_MyInteract"))
  (:Started
    (if (Utilities|IsValid (Variables|Default|GetTargetDoor))
      (Default|TryOpen (Variables|Default|GetTargetDoor)))))

(event Input|EnhancedActionEvents|EnhancedInputActionIA_MyJump
  (params (ActionValue :type Boolean) (ElapsedSeconds :type Float%20%28double-precision%29) (TriggeredSeconds :type Float%20%28double-precision%29) (InputAction :type Input%20Action%20Object%20Reference :default "/Game/Input/IA_MyJump.IA_MyJump"))
  (:Triggered
    (Character|Jump self))
  (:Completed
    (Character|StopJumping self)))

(event Game|Damage|EventAnyDamage
  (params (Damage :type Float%20%28single-precision%29) (DamageType :type Damage%20Type%20Object%20Reference) (InstigatedBy :type Controller%20Object%20Reference) (DamageCauser :type Actor%20Object%20Reference))
  (bind _returnvalue (Game|GetPlayerController 0))
  (Variables|Default|SetHealth (Math|Float|Clamp(Float) (- (Variables|Default|GetHealth) Damage) 0.0 (Variables|Default|GetMaxHealth)))
  (if (> (Variables|Default|GetHealth) 0.0)
    (bind _returnvalue_2 (UserInterface|CreateWidget "/Game/UI/WBP_DamageFlash.WBP_DamageFlash_C"))
    (UserInterface|Viewport|AddtoViewport _returnvalue_2 0)
    (Utilities|FlowControl|Delay 0.2)
    (Widget|RemovefromParent _returnvalue_2)
    (else
      (Utilities|FlowControl|DoOnce false
        (:Completed
          (Input|DisableInput self (Game|GetPlayerController 0))
          (Collision|SetCollisionEnabled (Variables|Collision|GetCapsuleComponent) "QueryOnly")
          (Physics|SetSimulatePhysics (Variables|Character|GetMesh) false)
          (Collision|SetCollisionProfileName (Variables|Character|GetMesh) "Ragdoll" true :!class /Script/Engine.PrimitiveComponent)
          (bind _returnvalue_3 (UserInterface|CreateWidget "/Game/UI/WBP_GameOver.WBP_GameOver_C"))
          (UserInterface|Viewport|AddtoViewport _returnvalue_3 0)
          (Variables|/Script/Engine.PlayerController|SetbShowMouseCursor _returnvalue true)
          (Input|SetInputModeUIOnly _returnvalue 0 "DoNotLock" false))))))

(event EventBeginPlay
  (Utilities|FlowControl|Sequence
    (:then_0
      (bind _asプレイヤーコントローラー (Utilities|Casting|CastToPlayerController (Pawn|GetController)))
      (Input|AddMappingContext (PlayerController|LocalPlayerSubsystems|GetEnhancedInputLocalPlayerSubsystem _asプレイヤーコントローラー) "/Game/Input/IMC_MyDefault.IMC_MyDefault" 0 "(bIgnoreAllPressedKeysUntilRelease=True,bForceImmediately=False,bNotifyUserSettings=False)")
      (bind _returnvalue (UserInterface|CreateWidget "/Game/UI/WBP_UI.WBP_UI_C"))
      (UserInterface|Viewport|AddtoViewport _returnvalue 0))
    (:then_1
      (bind _returnvalue_2 (Rendering|Material|CreateDynamicMaterialInstance (Variables|Character|GetMesh) 0 "/Game/Characters/Mannequins/Materials/Manny/MI_Manny_01_New.MI_Manny_01_New" "None" :!class /Script/Engine.PrimitiveComponent))
      (Variables|Default|SetHeadMat_Dynamic _returnvalue_2))))

(event Input|KeyboardEvents|V
  (params (Key :type Key%20Structure :default "None"))
  (bind _fps_camera (Variables|Default|GetFPS_Camera))
  (bind _tps_camera (Variables|Default|GetTPS_Camera))
  ;[0.15 0.15 0.15 0.5] カメラ切り替え
  (:Pressed
    (Utilities|FlowControl|FlipFlop
      (:A
        (Components|Activation|SetActive _fps_camera false false)
        (Components|Activation|SetActive _tps_camera true false)
        (Rendering|Material|SetScalarParameterValue (Variables|Default|GetHeadMat_Dynamic) "Opacity" 1.0 :!class /Script/Engine.MaterialInstanceDynamic))
      (:B
        (Components|Activation|SetActive _fps_camera true false)
        (Components|Activation|SetActive _tps_camera false false)
        (Rendering|Material|SetScalarParameterValue (Variables|Default|GetHeadMat_Dynamic) "Opacity" 0.0 :!class /Script/Engine.MaterialInstanceDynamic)))))

(fn ConstructionScript)