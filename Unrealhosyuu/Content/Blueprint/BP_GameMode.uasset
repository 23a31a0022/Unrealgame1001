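; Game mode that tracks the number of living enemies and spawns the clear key when none remain.
; EnemySpawned and EnemyDied raise or lower EnemyCount, then broadcast it through the OnEnemyCountChanged dispatcher.
; When a death brings the count to zero or below, BP_ClearKey spawns at the location passed with that death.
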(event Custom|EnemyDied
  (params (SpawnLocation :type Vector))
  (bind _output_get (Variables|Default|SetEnemyCount (- (Variables|Default|GetEnemyCount) 1)))
  (Default|CallOnEnemyCountChanged _output_get)
  (if (<= (Variables|Default|GetEnemyCount) 0)
    (Game|SpawnActorfromClass "/Game/Blueprint/BP_ClearKey.BP_ClearKey_C" (Math|Transform|MakeTransform SpawnLocation) "Undefined" "MultiplyWithRoot" 0 0)))

(event Custom|EnemySpawned
  (bind _output_get (Variables|Default|SetEnemyCount (+ (Variables|Default|GetEnemyCount) 1)))
  (Default|CallOnEnemyCountChanged _output_get))

(fn ConstructionScript)