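; BP_Door is an interactable door that can start locked and swings open on a timeline when the player tries it.
; On BeginPlay, an escape door unlocks on the game mode's all-enemies-defeated event, while other doors unlock when the player acquires a key.
; Its box overlap registers it as the player's target door and toggles the interact prompt with the lock state.
; TryOpen prints a locked message or rotates the door's yaw.
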(event OnComponentBeginOverlap(Box)
  (params (OverlappedComponent :type Primitive%20Component%20Object%20Reference) (OtherActor :type Actor%20Object%20Reference) (OtherComp :type Primitive%20Component%20Object%20Reference) (OtherBodyIndex :type Integer) (bFromSweep :type Boolean) (SweepResult :type Hit%20Result%20Structure%20%28by%20ref%29))
  (bind _asbp_player (Utilities|Casting|CastToBP_Player OtherActor))
  (Variables|/Game/Blueprint/BP_Player.BP_Player_C|SetTargetDoor _asbp_player self)
  (Default|ShowInteract _asbp_player (Variables|Default|GetIsLocked)))

(event OnComponentEndOverlap(Box)
  (params (OverlappedComponent :type Primitive%20Component%20Object%20Reference) (OtherActor :type Actor%20Object%20Reference) (OtherComp :type Primitive%20Component%20Object%20Reference) (OtherBodyIndex :type Integer))
  (bind _asbp_player (Utilities|Casting|CastToBP_Player OtherActor))
  (Variables|/Game/Blueprint/BP_Player.BP_Player_C|SetTargetDoor _asbp_player 0)
  (Default|HideInteract _asbp_player))

(event Custom|Unlock
  (Variables|Default|SetIsLocked false))

(event Custom|TryOpen
  (if (Variables|Default|GetIsLocked)
    (Development|PrintString "鍵がかかっている！")
    (else
      (bind _door (Timeline|タイムライン Play)
        (:Update
          (Transformation|SetRelativeRotation (Variables|Default|GetDoorPaul) (Math|Rotator|MakeRotator 0.0 0.0 _door) false false))))))

(event Custom|UnlockEscape
  (Variables|Default|SetIsLocked false))

(event EventBeginPlay
  (if (Variables|Default|GetIsEscapeDoor)
    (bind _asbp_game_mode (Utilities|Casting|CastToBP_GameMode (Game|GetGameMode)))
    (EventDispatchers|BindEventtoOnAllEnemiesDefeated _asbp_game_mode (delegate Custom|UnlockEscape))
    (else
      (bind _asbp_player (Utilities|Casting|CastToBP_Player (Game|GetPlayerCharacter 0)))
      (EventDispatchers|BindEventtoOnKeyAcquired _asbp_player (delegate Custom|Unlock)))))

(fn ConstructionScript)