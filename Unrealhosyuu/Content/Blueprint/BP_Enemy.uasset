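; BP_Enemy is an enemy character that takes hits and reports its spawn and death to BP_GameMode.
; On BeginPlay it notifies the game mode that it has spawned.
; Each TakeDamage call removes one Health; at zero or below, the mesh becomes a physics ragdoll, capsule collision turns off and EnemyDied receives its location.
; The trailing DoOnce follows the death report, so it does not guard against repeat calls.
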(event Custom|TakeDamage
  (Variables|Default|SetHealth (- (Variables|Default|GetHealth) 1))
  (if (<= (Variables|Default|GetHealth) 0)
    (Physics|SetSimulatePhysics (Variables|Character|GetMesh) true)
    (Collision|SetCollisionProfileName (Variables|Character|GetMesh) "Ragdoll" true :!class /Script/Engine.PrimitiveComponent)
    (Collision|SetCollisionEnabled (Variables|Collision|GetCapsuleComponent) "NoCollision")
    (bind _asbp_game_mode (Utilities|Casting|CastToBP_GameMode (Game|GetGameMode)))
    (Default|EnemyDied _asbp_game_mode (Transformation|GetActorLocation))
    (Utilities|FlowControl|DoOnce false)))

(event EventBeginPlay
  (bind _asbp_game_mode (Utilities|Casting|CastToBP_GameMode (Game|GetGameMode)))
  (Default|EnemySpawned _asbp_game_mode))

(fn ConstructionScript)